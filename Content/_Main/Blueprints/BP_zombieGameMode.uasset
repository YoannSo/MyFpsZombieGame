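; Game mode for a wave-based zombie shooter that runs from the first wave to a win screen after the last.
; Each wave spawns one randomly placed ammo crate and four zombies per wave number, split between two fixed spawn points.
; ZombieOnKill counts down the remaining zombies, then either shows the next wave UI and spawns after a short delay, or shows the win UI through the player character.
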(event `PlayerWin`
  (bind _asbp_first_person_character (cast `/Game/_Main/Blueprints/BP_FirstPersonCharacter` (`GameplayStatics.GetPlayerCharacter` 0)))
  (`/Game/_Main/Blueprints/BP_FirstPersonCharacter.ShowWinUi` _asbp_first_person_character))

(event `ZombieOnKill`
  (bind _result (`/Engine/EditorBlueprintResources/StandardMacros.DecrementInt` (`self.ZombieLeft`))
    (:`  `
      (if (== _result 0)
        (`self.NewWave`)))))

(event `NewWave`
  (if (== (`self.CurrentWave`) (`self.MaxWave`))
    (`self.PlayerWin`)
    (else
      (`/Engine/EditorBlueprintResources/StandardMacros.IncrementInt` (`self.CurrentWave`)
        (:`  `
          (bind _asbp_first_person_character (cast `/Game/_Main/Blueprints/BP_FirstPersonCharacter` (`GameplayStatics.GetPlayerCharacter` 0)))
          (`/Game/_Main/Blueprints/BP_FirstPersonCharacter.ShowWaveUI` _asbp_first_person_character (`self.CurrentWave`))
          (`KismetSystemLibrary.Delay` 5.0)
          (`self.SpawnZombie`))))))

(event `self.ReceiveBeginPlay`
  ;[1 1 1] start game
  (`self.StartGame`))

(event `StartGame`
  ;[1 1 1] start game
  (`self.SpawnZombie`))

(event `SpawnZombie`
  ;[1 1 1] spawn zombie
  (`self.SpawnAmmo`)
  (bind _output_get (set `self.ZombieTotal` (* (`self.CurrentWave`) 4)))
  (set `self.ZombieLeft` _output_get)
  (for _index (range (+ _output_get 1))
    (if (== _index (/ (`self.ZombieTotal`) 2))
      (break)
      (else
        (`|SpawnActorFromClass` "/Game/_Main/Zombie/BP_ZombieGirl.BP_ZombieGirl_C" (`self.SpawnLocation1`) "Undefined" "MultiplyWithRoot" null null))))
  (for _ (range 1 (+ (/ (`self.ZombieTotal`) 2) 1))
    (`|SpawnActorFromClass` "/Game/_Main/Zombie/BP_ZombieGirl.BP_ZombieGirl_C" (`self.SpawnLocation2`) "Undefined" "MultiplyWithRoot" null null)))

(event `SpawnAmmo`
  ;[1 1 1] spawn ammo crate
  (`|SpawnActorFromClass` "/Game/_Main/Blueprints/BP_AmmoPickUp.BP_AmmoPickUp_C" (`KismetMathLibrary.MakeTransform` (`|GetArrayItem` (`self.AmmoCrateLocation`) (`KismetMathLibrary.RandomInteger` 3))) "Undefined" "MultiplyWithRoot" null null))

(fn `UserConstructionScript`)