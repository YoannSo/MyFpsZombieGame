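; BP_ZombieGirl is a zombie enemy that chases and melees the player.
; It loops between AI MoveTo and an attack montage, whose notify triggers a sound and a sphere overlap that damages the first-person character.
; Seeing a pawn sets its walk speed.
; Point damage lowers health and plays a hit reaction or death, which relaxes collision, reports the kill to the zombie game mode and destroys the actor after a delay.
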(event `DeathEvent`
  ;[1 1 1] death event
  (set `self.IsDead` true)
  (`MovementComponent.StopMovementImmediately` (`self.CharacterMovement`))
  (`|PlayMontage` (`self.Mesh`) "/Game/_Main/Zombie/Animations/ZombieDyingMontage.ZombieDyingMontage"
    (:`then`
      (`PrimitiveComponent.SetCollisionResponseToChannel` (`self.CapsuleComponent`) "ECC_Pawn" "ECR_Overlap")
      (`PrimitiveComponent.SetCollisionEnabled` (`self.Mesh`) "NoCollision")
      (bind _asbp_zombie_game_mode (cast `/Game/_Main/Blueprints/BP_zombieGameMode` (`GameplayStatics.GetGameMode`)))
      (`/Game/_Main/Blueprints/BP_zombieGameMode.ZombieOnKill` _asbp_zombie_game_mode)
      (`KismetSystemLibrary.Delay` 10.0)
      (`self.K2_DestroyActor`))))

(event `self.ReceivePointDamage`
  (params (Damage :type "Float (single-precision)") (DamageType :type "DamageType Object Reference") (HitLocation :type "Vector Structure") (HitNormal :type "Vector Structure") (HitComponent :type "PrimitiveComponent Object Reference") (BoneName :type Name) (ShotFromDirection :type "Vector Structure") (InstigatedBy :type "Controller Object Reference") (DamageCauser :type "Actor Object Reference") (HitInfo :type "HitResult Structure (by ref)"))
  (bind _health (`self.Health`))
  ;[1 1 1] when taking damage
  (if (`self.IsDead`)
    _
    (elif (<= _health 0.0)
      (`self.DeathEvent`)
      (else
        (bind _output_get (set `self.Health` (- _health Damage)))
        (if (<= _output_get 0.0)
          (`self.DeathEvent`)
          (else
            (`|PlayMontage` (`self.Mesh`) "/Game/_Main/Zombie/Animations/ZombieHitMontage.ZombieHitMontage")))))))

(event `self.ReceiveBeginPlay`
  (`self.RunToPlayer`))

(event `self.PawnSensing.OnSeePawn`
  (params (Pawn :type "Pawn Object Reference"))
  (set `CharacterMovementComponent.MaxWalkSpeed` 360.0 (`self.CharacterMovement`)))

(event `RunToPlayer`
  ;[1 1 1] chase player
  (if (not (`self.IsDead`))
    (`|AIMoveTo` self (0.0 0.0 0.0) (`GameplayStatics.GetPlayerController` 0) 40.0
      (:`OnSuccess`
        (`self.AttackPlayer`))
      (:`OnFail`
        (`self.RunToPlayer`)))))

(event `AttackPlayer`
  ;[1 1 1] attack player
  (`|PlayMontage` (`self.Mesh`) "/Game/_Main/Zombie/Animations/ZombieAttackMontage.ZombieAttackMontage"
    (:`OnCompleted`
      (`self.RunToPlayer`))
    (:`OnNotifyBegin`
      (`GameplayStatics.PlaySoundAtLocation` "/Game/_Main/Sounds/AttackCue.AttackCue" (`self.K2_GetActorLocation`) (struct) 1.0 1.0 0.0 "/Game/MilitaryWeapSilver/Sound/Attenuation/WeaponShot_att.WeaponShot_att" null null null)
      (bind (_outactors _returnvalue) (`KismetSystemLibrary.SphereOverlapActors` (`SceneComponent.K2_GetComponentLocation` (`self.Arrow1`)) 80.0 (`|MakeArray` "ObjectTypeQuery3" :!type "EObjectTypeQuery Enum") "/Game/_Main/Blueprints/BP_FirstPersonCharacter.BP_FirstPersonCharacter_C" (`|MakeArray` self :!type "Actor Object Reference")))
      (if _returnvalue
        (for _array_element _outactors
          (`GameplayStatics.ApplyDamage` _array_element 20.0 (`self.GetController`) self "/Script/Engine.DamageType"))))))

(fn `UserConstructionScript`)